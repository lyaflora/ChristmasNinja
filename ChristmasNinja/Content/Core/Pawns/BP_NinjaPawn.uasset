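; Player pawn for touch swipe slicing, with movement deactivated and the mouse cursor shown.
; While Touch1 is held, Tick traces under the finger and feeds current and previous hit points plus swipe angle to a Niagara slice effect.
; An object-trace hit on a BP_Sliceable calls SliceAtLocation with a swipe-derived normal and impulse direction, then ends slicing until the next touch.
; Tick prints the angle for debugging; unconnected trace experiments remain.
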(event EventBeginPlay
  (Components|Activation|Deactivate (Variables|Default|GetMovementComponent))
  (Variables|/Script/Engine.PlayerController|SetbShowMouseCursor (Game|GetPlayerController 0) true))

(event EventTick
  (params (DeltaSeconds :type Float%20%28single-precision%29))
  (bind _returnvalue (Game|GetPlayerController 0))
  (bind _object_types (Variables|Default|GetObject%20Types))
  (bind _niagara (Variables|Default|GetNiagara))
  (bind (_hitresult _returnvalue_2) (Class|PlayerController|GetHitResultUnderFingerforObjects _returnvalue "Touch1" _object_types false))
  (bind (_hitresult_2 _returnvalue_3) (Class|PlayerController|GetHitResultUnderFingerbyChannel _returnvalue "Touch1" "TraceTypeQuery1" false))
  (bind (_bblockinghit _binitialoverlap _time _distance _location _impactpoint _normal _impactnormal _physmat _hitactor) (Collision|BreakHitResult _hitresult))
  (bind (_bblockinghit_2 _binitialoverlap_2 _time_2 _distance_2 _location_2 _impactpoint_2 _normal_2 _impactnormal_2 _physmat_2 _hitactor_2) (Collision|BreakHitResult _hitresult_2))
  (if (Variables|Default|GetbTouchHeld)
    (Development|PrintString (Utilities|String|ToString(Float) (Class|KismetMathLibrary|DegAcos (Math|Vector|DotProduct (Math|Vector|SelectVector (Math|Vector|RotateVector (Math|Vector|Normalize (- _location_2 (Variables|Default|GetPreviousHitLocation))) "0, 0,180.000000") (Math|Vector|Normalize (- _location_2 (Variables|Default|GetPreviousHitLocation))) (< (.Z (Math|Vector|BreakVector (Math|Vector|RotateVector (Math|Vector|Normalize (- _location_2 (Variables|Default|GetPreviousHitLocation))) "0, 0,90.000000"))) 0.0)) "0, 0,1.000000"))))
    (if _returnvalue_3
      (Effects|Components|ParticleSystem|SetVectorParameter _niagara "User.LastSliceLocation" (Variables|Default|GetPreviousHitLocation))
      (Effects|Components|ParticleSystem|SetVectorParameter _niagara "User.SliceLocation" _location_2)
      (Effects|Components|ParticleSystem|SetFloatParameter _niagara "User.SliceRotation" (Class|KismetMathLibrary|DegAcos (Math|Vector|DotProduct (Math|Vector|SelectVector (Math|Vector|RotateVector (Math|Vector|Normalize (- _location_2 (Variables|Default|GetPreviousHitLocation))) "0, 0,180.000000") (Math|Vector|Normalize (- _location_2 (Variables|Default|GetPreviousHitLocation))) (< (.Z (Math|Vector|BreakVector (Math|Vector|RotateVector (Math|Vector|Normalize (- _location_2 (Variables|Default|GetPreviousHitLocation))) "0, 0,90.000000"))) 0.0)) "0, 0,1.000000")))
      (if _returnvalue_2
        (bind _asbp_sliceable (Utilities|Casting|CastToBP_Sliceable _hitactor))
        (Default|SliceatLocation _asbp_sliceable _location (Math|Vector|SelectVector (Math|Vector|RotateVector (Math|Vector|RotateVector (Math|Vector|Normalize (- _location_2 (Variables|Default|GetPreviousHitLocation))) "0, 0,90.000000") "0, 0,180.000000") (Math|Vector|RotateVector (Math|Vector|Normalize (- _location_2 (Variables|Default|GetPreviousHitLocation))) "0, 0,90.000000") (< (.Z (Math|Vector|BreakVector (Math|Vector|RotateVector (Math|Vector|Normalize (- _location_2 (Variables|Default|GetPreviousHitLocation))) "0, 0,90.000000"))) 0.0)) (Math|Vector|SelectVector (Math|Vector|RotateVector (Math|Vector|Normalize (- _location_2 (Variables|Default|GetPreviousHitLocation))) "0, 0,180.000000") (Math|Vector|Normalize (- _location_2 (Variables|Default|GetPreviousHitLocation))) (< (.Z (Math|Vector|BreakVector (Math|Vector|RotateVector (Math|Vector|Normalize (- _location_2 (Variables|Default|GetPreviousHitLocation))) "0, 0,90.000000"))) 0.0)))
        (Variables|Default|SetbTouchHeld false))
      (Variables|Default|SetPreviousHitLocation _location_2))))

(event Input|TouchEvents|Touch1
  (params (Key :type Key%20Structure :default "None"))
  (bind _returnvalue (Game|GetPlayerController 0))
  (bind _niagara (Variables|Default|GetNiagara))
  (bind (_hitresult _returnvalue_2) (Class|PlayerController|GetHitResultUnderFingerbyChannel _returnvalue "Touch1" "TraceTypeQuery1" false))
  (bind (_bblockinghit _binitialoverlap _time _distance _location _impactpoint _normal _impactnormal _physmat _hitactor) (Collision|BreakHitResult _hitresult))
  (:Pressed
    (Variables|Default|SetbTouchHeld true)
    (Effects|Components|ParticleSystem|SetVectorParameter _niagara "User.SliceLocation" _location)
    (Components|Activation|Activate _niagara false)
    (if _returnvalue_2
      (Variables|Default|SetPreviousHitLocation _location)
      (Effects|Components|ParticleSystem|SetVectorParameter _niagara "User.LastSliceLocation" _location)
      (Effects|Components|ParticleSystem|SetFloatParameter _niagara "User.SliceRotation" (Class|KismetMathLibrary|DegAcos (Math|Vector|DotProduct (Math|Vector|SelectVector (Math|Vector|RotateVector (Math|Vector|Normalize (- _location (Variables|Default|GetPreviousHitLocation))) "0, 0,180.000000") (Math|Vector|Normalize (- _location (Variables|Default|GetPreviousHitLocation))) (< (.Z (Math|Vector|BreakVector (Math|Vector|RotateVector (Math|Vector|Normalize (- _location (Variables|Default|GetPreviousHitLocation))) "0, 0,90.000000"))) 0.0)) "0, 0,1.000000")))))
  (:Released
    (Variables|Default|SetbTouchHeld false)
    (Components|Activation|Deactivate _niagara)))

(fn ConstructionScript)