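; BP_Sliceable is a physics-launched object that can be sliced in two and destroys itself on a short timer.
; The construction script copies a sample static mesh into a procedural mesh with collision and a material.
; BeginPlay starts the resettable timer and applies an upward impulse with configurable Y velocity.
; SliceatLocation cuts along a given plane with a capped face, sets both halves to WorldStatic collision and reapplies the pre-cut velocity as impulses.
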(event Custom|Slice%20at%20Location
  (params (Location :type Vector) (Normal :type Vector :default "0,0,1.000000") (ImpulseDirection :type Vector :default "300.000000,300.000000,300.000000"))
  (bind _proceduralmesh (Variables|Default|GetProceduralMesh))
  (bind _returnvalue (Physics|GetPhysicsLinearVelocity _proceduralmesh "None"))
  (bind _outotherhalfprocmesh (Class|KismetProceduralMeshLibrary|SliceProceduralMesh _proceduralmesh Location Normal true "CreateNewSectionForCap" (Rendering|Material|GetMaterial _proceduralmesh 0)))
  (Collision|SetCollisionObjectType _outotherhalfprocmesh "ECC_WorldStatic")
  (Collision|SetCollisionObjectType _proceduralmesh "ECC_WorldStatic")
  (Physics|SetSimulatePhysics _outotherhalfprocmesh true)
  (Class|PrimitiveComponent|SetMassScale (Variables|Default|GetProceduralMesh) "None" 0.01)
  (Physics|AddImpulse _outotherhalfprocmesh _returnvalue "None" true)
  (Physics|AddImpulse _proceduralmesh _returnvalue "None" true))

(event Custom|Destroy
  (Actor|DestroyActor))

(event Custom|ResetTimer
  (Utilities|Time|ClearandInvalidateTimerbyHandle (Variables|Default|GetDestroyTimer))
  (bind _returnvalue (Utilities|Time|SetTimerbyEvent (delegate Custom|Destroy) 5.0))
  (Variables|Default|SetDestroyTimer _returnvalue))

(event EventBeginPlay
  (CallFunction|ResetTimer)
  (Physics|AddImpulse (Variables|Default|GetProceduralMesh) (Math|Vector|MakeVector 0.0 (Variables|Default|GetInitialImpulseY) 4.5e+02) "None" true))

(event EventTick
  (params (DeltaSeconds :type Float%20%28single-precision%29)))

(fn ConstructionScript
  (bind _proceduralmesh (Variables|Default|GetProceduralMesh))
  (Components|StaticMesh|SetStaticMesh (Variables|Default|GetStaticMesh) (Variables|Default|GetStaticMeshSample))
  (Class|KismetProceduralMeshLibrary|CopyProceduralMeshfromStaticMeshComponent (Variables|Default|GetStaticMesh) 0 _proceduralmesh true)
  (Rendering|Material|SetMaterial _proceduralmesh 0 (Variables|Default|GetMaterialSample)))